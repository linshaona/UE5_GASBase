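; Player primary attack Gameplay Ability that plays a melee montage and damages the actors it hits.
; A FlipFlop alternates between the A and B montages, and the ability ends when the montage completes, blends out or is interrupted or cancelled.
; In parallel, it waits for the Primary gameplay event, runs a hitbox overlap test, sends hit reacts and applies GE_PlayerDamage at ability level to each overlapped actor.
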(event `self.K2_ActivateAbility`
  (bind _returnvalue (`self.GetAbilitySystemComponentFromActorInfo`))
  (`|ExecutionSequence`
    (:`then_0`
      ;[0.01492 0.03096 0.15 0.5] Play Attack Montage
      (`/Engine/EditorBlueprintResources/StandardMacros.FlipFlop`
        (:`A`
          (`AbilityTask_PlayMontageAndWait.CreatePlayMontageAndWaitProxy` "None" "/Game/GASBase/Characters/PlayerCharacter/Animations/GB_Primary_A_Montage.GB_Primary_A_Montage"
            (:`OnCompleted`
              _)
            (:`OnBlendOut`
              _)
            (:`OnInterrupted`
              _)
            (:`OnCancelled`
              _))
          (`self.K2_EndAbility`))
        (:`B`
          (`AbilityTask_PlayMontageAndWait.CreatePlayMontageAndWaitProxy` "None" "/Game/GASBase/Characters/PlayerCharacter/Animations/GB_Primary_B_Montage.GB_Primary_B_Montage"
            (:`OnCompleted`
              _)
            (:`OnBlendOut`
              _)
            (:`OnInterrupted`
              _)
            (:`OnCancelled`
              _))
          (`self.K2_EndAbility`))))
    (:`then_1`
      (`AbilityTask_WaitGameplayEvent.WaitGameplayEvent` (struct :`TagName` "CTags.Events.Player.Primary") null
        (:`EventReceived`
          (bind _returnvalue_2 (`self.HitBoxOverlapTest`))
          (`self.SendHitReactEventToActor` _returnvalue_2)
          (for _array_element _returnvalue_2
            (`AbilitySystemComponent.BP_ApplyGameplayEffectSpecToTarget` _returnvalue (`AbilitySystemComponent.MakeOutgoingSpec` :`self` _returnvalue :`GameplayEffectClass` "/Game/GASBase/AbilitySystem/GameplayEffects/Player/GE_PlayerDamage.GE_PlayerDamage_C" :`Level` (`KismetMathLibrary.Conv_IntToDouble` (`self.GetAbilityLevel`))) (`AbilitySystemBlueprintLibrary.GetAbilitySystemComponent` _array_element))))))))
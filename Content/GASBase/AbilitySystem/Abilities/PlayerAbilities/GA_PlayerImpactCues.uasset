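; Player gameplay ability that listens for hit-react and death gameplay events and triggers the matching responses.
; On hit react it executes the HitReact gameplay cue twice, once plain and once with the event's instigator and optional object as parameters.
; On death it activates abilities tagged Death through the ability system component, allowing remote activation.
; It never calls EndAbility, so both waits act as persistent listeners.
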(event `self.K2_ActivateAbility`
  (`|ExecutionSequence`
    (:`then_0`
      (bind (_asynctaskproxy _payload) (`AbilityTask_WaitGameplayEvent.WaitGameplayEvent` (struct :`TagName` "CTags.Events.Player.HitReact") null)
        (:`EventReceived`
          (`self.K2_ExecuteGameplayCue` (struct :`TagName` "GameplayCue.HitReact"))
          (bind (_eventtag _instigator _target _optionalobject) (break `GameplayEventData` _payload))
          (`self.K2_ExecuteGameplayCueWithParams` (struct :`TagName` "GameplayCue.HitReact") (`AbilitySystemBlueprintLibrary.MakeGameplayCueParameters` 0.0 0.0 (struct) (struct) (struct) (struct) (struct) (0.0 0.0 0.0) (0.0 0.0 0.0) _instigator null _optionalobject)))))
    (:`then_1`
      (`AbilityTask_WaitGameplayEvent.WaitGameplayEvent` (struct :`TagName` "CTags.Events.Player.Death") null
        (:`EventReceived`
          (`AbilitySystemComponent.TryActivateAbilitiesByTag` (`self.GetAbilitySystemComponentFromActorInfo`) (`BlueprintGameplayTagLibrary.MakeGameplayTagContainerFromTag` (`BlueprintGameplayTagLibrary.MakeLiteralGameplayTag` (struct :`TagName` "CTags.CAbilities.Death"))) true))))))
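; Gameplay Ability that listens for health changes on the owner and triggers death when the value reaches zero.
; On activation it starts a ListenForAttributeChange async task on the owner's Ability System Component and stores the task.
; When the new value is zero or below, it tries to activate abilities tagged as Death, allowing remote activation.
; The stored task is ended when the ability ends.
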(event `self.K2_ActivateAbility`
  (bind (_asynctaskproxy _attribute _newvalue) (`CAttributeChangeTask.ListenForAttributeChange` (`self.GetAbilitySystemComponentFromActorInfo`) (struct :`AttributeName` "Health" :`Attribute` "/Script/GASBase.CAttributeSet:Health" :`AttributeOwner` "/Script/CoreUObject.Class'/Script/GASBase.CAttributeSet'"))
    (:`then`
      (set `self.AttributeChangeTask` _asynctaskproxy))
    (:`OnAttributeChanged`
      (if (<= _newvalue 0.0)
        (`AbilitySystemComponent.TryActivateAbilitiesByTag` (`self.GetAbilitySystemComponentFromActorInfo`) (`BlueprintGameplayTagLibrary.MakeGameplayTagContainerFromTag` (`BlueprintGameplayTagLibrary.MakeLiteralGameplayTag` (struct :`TagName` "CTags.CAbilities.Death"))) true)))))

(event `self.K2_OnEndAbility`
  (params (bWasCancelled :type Boolean))
  (bind _attributechangetask (`self.AttributeChangeTask`)
    (:`then`
      (`CAttributeChangeTask.EndTask` _attributechangetask))
    (:`else`)))
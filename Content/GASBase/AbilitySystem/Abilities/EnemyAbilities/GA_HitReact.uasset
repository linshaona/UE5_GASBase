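; Enemy hit reaction gameplay ability that, once activated, listens for the HitReact gameplay event and never ends itself in this graph.
; On each event it skips dead owners, caches vectors from the instigator and resolves a hit direction name relative to the avatar's forward.
; That name doubles as the section to jump to in a single hit react montage.
; Optional debug prints show the instigator and direction.
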(event `self.K2_ActivateAbility`
  (bind (_asynctaskproxy _payload) (`AbilityTask_WaitGameplayEvent.WaitGameplayEvent` (struct :`TagName` "CTags.Events.Enemy.HitReact") null)
    (:`EventReceived`
      (if (not (`GameplayTagAssetInterface.HasMatchingGameplayTag` (`self.GetAbilitySystemComponentFromActorInfo`) (struct :`TagName` "CTags.Status.Dead")))
        (`self.PrintDebugEventReceived` _payload)
        (`self.CacheHitDirectionVectors` (`.Instigator` (break `GameplayEventData` _payload)))
        (`|ExecutionSequence`
          (:`then_0`
            ; Cache Hit Direction Name
            (bind _output_get (set `self.HitDirectionName` (`CBlueprintLibrary.GetHitDirectionName` (`CBlueprintLibrary.GetHitDirection` (`self.AvatarForward`) (`self.ToInstigator`)))))
            ; Debug for Hit Direction
            (`self.bDrawDebug`
              (:`then`
                (`KismetSystemLibrary.PrintString` (`KismetStringLibrary.Conv_NameToString` _output_get)))
              (:`else`)))
          (:`then_1`
            ; Play Montage and Jump to the corrent Hit React Montage Section
            (`AbilityTask_PlayMontageAndWait.CreatePlayMontageAndWaitProxy` "None" (`self.HitReactMontage`)
              (:`then`
                (`self.MontageJumpToSection` (`self.HitDirectionName`))))))))))

(fn `PrintDebugEventReceived`
  (params (GameplayEventData :type "GameplayEventData Structure (by ref)"))
  (`self.bDrawDebug`
    (:`then`
      (`KismetSystemLibrary.PrintString` (`KismetStringLibrary.Concat_StrStr` "GA_HitReact:Received Event from:" (`KismetSystemLibrary.GetDisplayName` (`.Instigator` (break `GameplayEventData` GameplayEventData))))))
    (:`else`)))
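; Gameplay ability for enemy death that plays a death montage, applies the death effect, then respawns the character in place of destroying it.
; When the montage completes, is interrupted or is cancelled, it removes the effect granting the Dead status tag.
; The server then resets attributes and moves the character to a player start.
; The ability ends before calling the character's respawn handler, which is not authority-gated.
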(event `self.K2_ActivateAbility`
  (bind _returnvalue (`self.GetAbilitySystemComponentFromActorInfo`))
  (`AbilityTask_PlayMontageAndWait.CreatePlayMontageAndWaitProxy` "None" (`self.DeathMontage`)
    (:`then`
      (`AbilitySystemComponent.BP_ApplyGameplayEffectSpecToSelf` _returnvalue (`AbilitySystemComponent.MakeOutgoingSpec` :`self` _returnvalue :`GameplayEffectClass` "/Game/GASBase/AbilitySystem/GameplayEffects/GE_Death.GE_Death_C" :`Level` 1.0)))
    (:`OnCompleted`
      (`self.RespawnCharacter` :!label _label))
    (:`OnInterrupted`
      (goto _label))
    (:`OnCancelled`
      (goto _label))))

(event `RespawnCharacter`
  (`|ExecutionSequence`
    (:`then_0`
      (`self.BP_RemoveGameplayEffectFromOwnerWithGrantedTags` (struct :`GameplayTags` (struct :`(TagName` "CTags.Status.Dead"))) 1))
    (:`then_1`
      ; Cache CBaseCharacter
      (bind _ascbase_character (cast `CBaseCharacter` (`self.GetAvatarActorFromActorInfo`)))
      (set `self.CBaseCharacter` _ascbase_character))
    (:`then_2`
      ; Server only
      (`self.K2_HasAuthority`
        (:`True`
          (`|ExecutionSequence`
            (:`then_1`
              ;; Reset Attributes
              (bind _cbasecharacter (`self.CBaseCharacter`)
                (:`then`
                  (`CBaseCharacter.ResetAttributes` _cbasecharacter))
                (:`else`)))
            (:`then_2`
              ;; "Respawn" the Character
              (bind _cbasecharacter_2 (`self.CBaseCharacter`)
                (:`then`
                  (`Actor.K2_SetActorLocation` (`self.CBaseCharacter`) (`Actor.K2_GetActorLocation` (`GameModeBase.K2_FindPlayerStart` (`GameplayStatics.GetGameMode`) (`Pawn.GetController` _cbasecharacter_2) "")) false false))
                (:`else`)))))))
    (:`then_3`
      (`self.K2_EndAbility`))
    (:`then_4`
      ; Handle Respawn
      (bind _cbasecharacter_3 (`self.CBaseCharacter`)
        (:`then`
          (`CBaseCharacter.HandleRespawn` _cbasecharacter_3))
        (:`else`)))))
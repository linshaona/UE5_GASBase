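; Gameplay Ability for enemy melee attacks in a GAS setup.
; If the avatar is dead it sends an EndAttack event and ends; otherwise it plays a random attack montage and ends when that completes or is cancelled.
; In parallel it waits once for a MeleeTraceHit event and deals SetByCaller melee damage with impact particles to the hit target.
; Ending the ability always sends EndAttack to the avatar.
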(event `self.K2_ActivateAbility`
  (if (`GameplayTagAssetInterface.HasMatchingGameplayTag` (`self.GetAbilitySystemComponentFromActorInfo`) (struct :`TagName` "CTags.Status.Dead"))
    (`AbilitySystemBlueprintLibrary.SendGameplayEventToActor` (`self.GetAvatarActorFromActorInfo`) (struct :`TagName` "CTags.CAbilities.Enemy.EndAttack"))
    (`self.K2_EndAbility`)
    (else
      (`|ExecutionSequence`
        (:`then_0`
          ; Play Attack Montage
          (`AbilityTask_PlayMontageAndWait.CreatePlayMontageAndWaitProxy` "None" (`KismetArrayLibrary.Array_Random` (`self.AttackMontages`))
            (:`OnCompleted`
              _)
            (:`OnInterrupted`
              _)
            (:`OnCancelled`
              _))
          (`self.K2_EndAbility`))
        (:`then_1`
          (bind (_asynctaskproxy _payload) (`AbilityTask_WaitGameplayEvent.WaitGameplayEvent` (struct :`TagName` "CTags.Events.Enemy.MeleeTraceHit") null true)
            (:`EventReceived`
              (`CBlueprintLibrary.SendDamageEventToPlayer` (`.Target` (break `GameplayEventData` _payload)) (`self.Damage Effect`) _payload (`BlueprintGameplayTagLibrary.MakeLiteralGameplayTag` (struct :`TagName` "CTags.SetByCaller.Melee")) 10.0 (`self.ImpactParticles`)))))))))

(event `self.K2_OnEndAbility`
  (params (bWasCancelled :type Boolean))
  (`AbilitySystemBlueprintLibrary.SendGameplayEventToActor` (`self.GetAvatarActorFromActorInfo`) (struct :`TagName` "CTags.CAbilities.Enemy.EndAttack")))